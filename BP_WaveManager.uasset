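; BP_WaveManager is a wave manager that spawns enemies at a path's start cube on a repeating timer.
; UpdateWave counts down by the supplied delta, spawns a BP_Enemy every four seconds, then calls AdvanceEnemies, which is still an empty stub.
; BeginPlay calls GetLength on a valid Path but sets PathLength to zero.
; Tick is disabled and nothing here calls UpdateWave.
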(event EventBeginPlay
  (bind _path (Variables|Default|GetPath)
    (:then
      (Default|GetLength _path)
      (Variables|Default|SetPathLength 0.0))
    (:else)))

(event Collision|EventActorBeginOverlap
  (params (OtherActor :type Actor%20Object%20Reference)))

(event EventTick
  (params (DeltaSeconds :type Float%20%28single-precision%29)))

(fn ConstructionScript)

(fn UpdateWave
  (params (Delta :type Float%20%28double-precision%29))
  (Utilities|FlowControl|Sequence
    (:then_0
      (bind _output_get (Variables|Default|SetTimeUntilEnemy (- (Variables|Default|GetTimeUntilEnemy) Delta)))
      (if (< _output_get 0.0)
        (Variables|Default|SetTimeUntilEnemy 4.0)
        (Game|SpawnActorfromClass "/Game/BP_Enemy.BP_Enemy_C" (Math|Conversions|ToTransform(Vector) (Transformation|GetWorldLocation (Variables|/Game/BP_Path.BP_Path_C|GetCube1 (Variables|Default|GetPath)))) "Undefined" "MultiplyWithRoot" 0 0)))
    (:then_1
      (CallFunction|AdvanceEnemies Delta))))

(fn AdvanceEnemies
  (params (Delta :type Float%20%28double-precision%29)))